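; AI fireball projectile that damages the player character on overlap.
; Overlapping a BP_PlayerCharacter subtracts a fixed amount from its Health, plays a hit montage on it, spawns an explosion emitter and destroys the projectile.
; It then calls the player's Death when Health reaches zero or below.
; Health is edited directly rather than through Apply Damage, and other overlapping actors are ignored.
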(event `self.ReceiveActorBeginOverlap`
  (params (OtherActor :type "Actor Object Reference"))
  (bind _asbp_player_character (cast `/Game/CORE/FlexibleCombatSystem/Blueprints/BP_PlayerCharacter` OtherActor))
  (bind _health (`/Game/CORE/FlexibleCombatSystem/Blueprints/BP_PlayerCharacter.Health` _asbp_player_character))
  (set `/Game/CORE/FlexibleCombatSystem/Blueprints/BP_PlayerCharacter.Health` (- _health 15) _asbp_player_character)
  (`Character.PlayAnimMontage` _asbp_player_character "/Game/CORE/FlexibleCombatSystem/Montages/M_HitImpact.M_HitImpact" 1.0 "None")
  (`GameplayStatics.SpawnEmitterAtLocation` "/Game/Assets/StarterContent/Particles/P_Explosion.P_Explosion" (`self.K2_GetActorLocation`))
  (`self.K2_DestroyActor`)
  (if (<= _health 0)
    (`/Game/CORE/FlexibleCombatSystem/Blueprints/BP_PlayerCharacter.Death` _asbp_player_character)))

(fn `UserConstructionScript`)