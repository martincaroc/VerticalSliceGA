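; Melee enemy character that chases and attacks sensed characters with a staff.
; PawnSensing triggers lock-on, staff equip and a looping AI MoveTo-and-combo attack, with retriggerable delays sheathing the weapon later.
; Equip and sheathe macros play montages, reattach the staff between sockets and notify the AnimInstance.
; Staff overlaps send hit messages; hits from Character_Human play a reaction montage, and Block input plays a block montage while armed.
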(event `self.PawnSensing.OnSeePawn`
  (params (Pawn :type "Pawn Object Reference"))
  (bind _sm_stf_staffofancients (`self.SM_Stf_StaffofAncients`))
  (bind _sm_stf_staffofancients_2 (`self.SM_Stf_StaffofAncients`))
  ;[1 1 1] IA
  (bind _ascharacter (cast `Character` Pawn))
  (`self.LockOn` true _ascharacter)
  (if (`self.Melee_weapon_eqquiped`) :!label _label
    (`KismetSystemLibrary.RetriggerableDelay` 5.0)
    (if (`self.Melee_weapon_eqquiped`)
      (`self.PlayAnimMontage` "/Game/Personaje/Blueprints/Animations/Combat/Standing_Disarm_Over_Shoulder__1__Montage.Standing_Disarm_Over_Shoulder__1__Montage")
      (`KismetSystemLibrary.Delay` 0.5)
      (set `self.Melee_weapon_eqquiped` false)
      (message `/Game/Personaje/Blueprints/BPI_Character.ToggleMeleeWeapon` (`SkeletalMeshComponent.GetAnimInstance` (`self.Mesh`)) false)
      (`SceneComponent.K2_AttachToComponent` _sm_stf_staffofancients_2 (`self.Mesh`) "WeaponIdle" "KeepWorld" "KeepWorld" "KeepWorld" true)
      (`KismetSystemLibrary.MoveComponentTo` _sm_stf_staffofancients_2))
    (else
      (`self.PlayAnimMontage` "/Game/Personaje/Blueprints/Animations/Combat/Unarmed_Equip_Over_Shoulder__1__Montage.Unarmed_Equip_Over_Shoulder__1__Montage")
      (`KismetSystemLibrary.Delay` 0.4)
      (set `self.Melee_weapon_eqquiped` true)
      (message `/Game/Personaje/Blueprints/BPI_Character.ToggleMeleeWeapon` (`SkeletalMeshComponent.GetAnimInstance` (`self.Mesh`)) true)
      (`SceneComponent.K2_AttachToComponent` _sm_stf_staffofancients (`self.Mesh`) "WeaponAttack" "KeepWorld" "KeepWorld" "KeepWorld" true)
      (`KismetSystemLibrary.MoveComponentTo` _sm_stf_staffofancients)
      (`|AIMoveTo` self (0.0 0.0 0.0) _ascharacter 75.0 :!label _label_2
        (:`then`
          (`KismetSystemLibrary.RetriggerableDelay` 10.0)
          (goto _label))
        (:`OnSuccess`
          (`KismetSystemLibrary.Delay` 0.2)
          (`self.PlayAnimMontage` "/Game/Personaje/Blueprints/Animations/Combat/Standing_Melee_Combo_Attack_Ver__3_Montage.Standing_Melee_Combo_Attack_Ver__3_Montage" 0.8)
          (`KismetSystemLibrary.Delay` 1.5)
          (goto _label_2))
        (:`OnFail`
          (`KismetSystemLibrary.Delay` 5.0)
          (goto _label_2))))))

(event `InputAction|Block`
  (params (Key :type "Key Structure"))
  ;[1 1 1] Block
  (:`Pressed`
    (set `self.Block` true)
    (if (`self.Melee_weapon_eqquiped`)
      (if (`self.Block`)
        (`self.PlayAnimMontage` "/Game/Personaje/Blueprints/Animations/Combat/Standing_Block_Idle__2__Montage.Standing_Block_Idle__2__Montage"))))
  (:`Released`
    (set `self.Block` true)
    (`self.StopAnimMontage` "/Game/Personaje/Blueprints/Animations/Combat/Standing_Block_Idle__2__Montage.Standing_Block_Idle__2__Montage")))

(event `self.SM_Stf_StaffofAncients.OnComponentBeginOverlap`
  (params (OverlappedComponent :type "PrimitiveComponent Object Reference") (OtherActor :type "Actor Object Reference") (OtherComp :type "PrimitiveComponent Object Reference") (OtherBodyIndex :type Integer) (bFromSweep :type Boolean) (SweepResult :type "HitResult Structure (by ref)"))
  (if (not (== OtherActor self))
    (`KismetSystemLibrary.PrintString` (`KismetSystemLibrary.GetDisplayName` OtherActor) true true (struct :`R` 1.0 :`G` 0.008603 :`A` 1.0) 1.0)
    (message `/Game/Personaje/Blueprints/BPI_Damageable.OnWeaponHit` OtherActor self)))

(event `/Game/Personaje/Blueprints/BPI_Damageable.OnWeaponHit`
  (params (`Source Actor` :type "Actor Object Reference"))
  (cast `/Game/Personaje/Blueprints/Character_Human` `Source Actor`)
  (`|PlayMontage` null "/Game/Personaje/Blueprints/Animations/Combat/Standing_React_Large_From_Right__1__Montage.Standing_React_Large_From_Right__1__Montage"))

(fn `UserConstructionScript`)