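; BP_FireballProjectile is a fireball projectile that damages BP_EnemyAI actors it overlaps.
; On a sphere overlap with an enemy it applies point damage, random between WeaponDamage and a fixed maximum, with the player character as damage causer.
; It then plays an impact sound and destroys itself.
; Any overlap also reaches a delayed destroy for non-enemy contacts, so a fireball that overlaps nothing gets no cleanup from this graph.
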(event `self.Sphere.OnComponentBeginOverlap`
  (params (OverlappedComponent :type "PrimitiveComponent Object Reference") (OtherActor :type "Actor Object Reference") (OtherComp :type "PrimitiveComponent Object Reference") (OtherBodyIndex :type Integer) (bFromSweep :type Boolean) (SweepResult :type "HitResult Structure (by ref)"))
  (`|ExecutionSequence`
    (:`then_0`
      (bind _asbp_enemy_ai (cast `/Game/CORE/FlexibleCombatSystem/Blueprints/AI/BP_EnemyAI` OtherActor))
      (`GameplayStatics.ApplyPointDamage` _asbp_enemy_ai (`KismetMathLibrary.RandomFloatInRange` (`self.WeaponDamage`) 60.0) (`.ImpactPoint` (`GameplayStatics.BreakHitResult` SweepResult)) SweepResult null (cast `/Game/CORE/FlexibleCombatSystem/Blueprints/BP_PlayerCharacter` (`GameplayStatics.GetPlayerCharacter` 0) :!pure true))
      (`GameplayStatics.PlaySoundAtLocation` "/Game/Mariano/SoundEfects/Cue_Sounds/Fireball_impact_Cue.Fireball_impact_Cue" (`self.K2_GetActorLocation` _asbp_enemy_ai) (struct) 1.0 1.0 0.0 null null null)
      (`self.K2_DestroyActor`))
    (:`then_1`
      (`KismetSystemLibrary.Delay` 2.5)
      (`self.K2_DestroyActor`))))

(fn `UserConstructionScript`)