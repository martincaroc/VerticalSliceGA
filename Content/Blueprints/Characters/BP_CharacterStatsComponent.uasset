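; BP_CharacterStatsComponent is a component that holds a character's health and coin stats.
; GainHealth adds an amount to Health and clamps it between zero and HealthMax, while GainCoins adds to Coins and keeps the total from going negative.
; Both functions print the new value on screen with Spanish labels.
; The event graph has no active logic.
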(fn `GainCoins`
  (params (`Coin to Gain` :type Integer))
  (bind _output_get (set `self.Coins` (`KismetMathLibrary.Max` (+ `Coin to Gain` (`self.Coins`)))))
  (`KismetSystemLibrary.PrintString` (`KismetStringLibrary.Concat_StrStr` "Monedas Actuales: " (`KismetStringLibrary.Conv_IntToString` _output_get))))

(fn `GainHealth`
  (params (`Health To Gain` :type "Float (double-precision)"))
  (bind _output_get (set `self.Health` (`KismetMathLibrary.FClamp` (+ `Health To Gain` (`self.Health`)) 0.0 (`self.HealthMax`))))
  (`KismetSystemLibrary.PrintString` (`KismetStringLibrary.Concat_StrStr` "Vida Actual:" (`KismetStringLibrary.Conv_DoubleToString` _output_get))))