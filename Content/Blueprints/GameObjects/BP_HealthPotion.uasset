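; Health potion pickup that restores health to the actor that collects it.
; On pickup, it looks up the collector's BP_CharacterStatsComponent and, if valid, calls GainHealth with HealthToGive.
; It then calls the parent PickedUp event, which according to the node comment shows who collided and destroys the object.
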(event `self.ReceiveTick`
  (params (DeltaSeconds :type "Float (single-precision)"))
  (`parent.ReceiveTick` DeltaSeconds))

(event `self.PickedUp`
  (params (ActorThatPickedThis :type "Actor Object Reference"))
  (bind _returnvalue (`self.GetComponentByClass` ActorThatPickedThis "/Game/Blueprints/Characters/BP_CharacterStatsComponent.BP_CharacterStatsComponent_C"))
  ;[0.4688 0.4688 0.4688] Si el actor es válido, llama la función para Sumar vida
  (`|ExecutionSequence`
    (:`then_0`
      (`/Engine/EditorBlueprintResources/StandardMacros.IsValid` _returnvalue
        (:`Is Valid`
          (`/Game/Blueprints/Characters/BP_CharacterStatsComponent.GainHealth` _returnvalue (`self.HealthToGive`)))))
    (:`then_1`
      ;[0.4219 0.4219 0.4219] Muestra quien Colisiono si es válido, y destruye el objeto
      (`parent.PickedUp` ActorThatPickedThis))))

(fn `UserConstructionScript`
  (`parent.UserConstructionScript`))