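; BP_BlockToggle is a demo room switch that toggles the BlockUp flag on a referenced dummy.
; Overlap of its Box by BP_PlayerCharacter drives a FlipFlop that alternately sets the flag on and off, swapping the mesh's two materials between green and red to match.
; A DoOnce that resets after a one-second delay debounces repeated overlaps.
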(event `self.Box.OnComponentBeginOverlap`
  (params (OverlappedComponent :type "PrimitiveComponent Object Reference") (OtherActor :type "Actor Object Reference") (OtherComp :type "PrimitiveComponent Object Reference") (OtherBodyIndex :type Integer) (bFromSweep :type Boolean) (SweepResult :type "HitResult Structure (by ref)"))
  (bind _staticmesh (`self.StaticMesh`))
  (bind _dummy_ref (`self.Dummy_Ref`))
  (cast `/Game/CORE/FlexibleCombatSystem/Blueprints/BP_PlayerCharacter` OtherActor)
  (`/Engine/EditorBlueprintResources/StandardMacros.DoOnce` false :!label _label
    (:`Completed`
      (`/Engine/EditorBlueprintResources/StandardMacros.FlipFlop`
        (:`A`
          (`PrimitiveComponent.SetMaterial` _staticmesh 0 "/Game/CORE/FlexibleCombatSystem/DemoRoom/Materials/M_Green.M_Green")
          (`PrimitiveComponent.SetMaterial` _staticmesh 1 "/Game/CORE/FlexibleCombatSystem/DemoRoom/Materials/M_Green.M_Green")
          (set `/Game/CORE/FlexibleCombatSystem/Blueprints/AI/TrainingDummys/BP_HitDummy.BlockUp` true _dummy_ref))
        (:`B`
          (`PrimitiveComponent.SetMaterial` _staticmesh 0 "/Game/CORE/FlexibleCombatSystem/DemoRoom/Materials/M_Red.M_Red")
          (`PrimitiveComponent.SetMaterial` _staticmesh 1 "/Game/CORE/FlexibleCombatSystem/DemoRoom/Materials/M_Red.M_Red")
          (set `/Game/CORE/FlexibleCombatSystem/Blueprints/AI/TrainingDummys/BP_HitDummy.BlockUp` false _dummy_ref)))
      (`KismetSystemLibrary.Delay` 1.0)
      (`self.Reset`))))

(event `Reset`
  (goto _label :!via `Reset`))

(fn `UserConstructionScript`)